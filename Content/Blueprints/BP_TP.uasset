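; BP_TP is a teleporter pad that moves the player to another BP_TP when a TopDownCharacter overlaps its Box while Active.
; It deactivates every BP_TP in the level, itself included, and teleports player 0 to each other pad in turn, so the last successful teleport sets the destination.
; It then calls DepopPopTp on the overlapping character; nothing here sets Active back to true.
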(event OnComponentBeginOverlap(Box)
  (params (OverlappedComponent :type Primitive%20Component%20Object%20Reference) (OtherActor :type Actor%20Object%20Reference) (OtherComp :type Primitive%20Component%20Object%20Reference) (OtherBodyIndex :type Integer) (bFromSweep :type Boolean) (SweepResult :type Hit%20Result%20Structure%20%28by%20ref%29))
  (bind _astop_down_character (Utilities|Casting|CastToTopDownCharacter OtherActor))
  (if (Variables|Default|Getactive)
    (bind _outactors (Actor|GetAllActorsOfClass "BP_TP_C"))
    (for _array_element _outactors
      (Variables|BP_TP_C|Setactive _array_element false)
      (if (not (== _array_element self))
        (Transformation|Teleport (Game|GetPlayerCharacter 0) (Transformation|GetActorLocation _array_element) "0, 0, 0")))
    (Default|DepopPopTp _astop_down_character)))

(event EventBeginPlay)

(event Collision|EventActorBeginOverlap
  (params (OtherActor :type Actor%20Object%20Reference)))

(event EventTick
  (params (DeltaSeconds :type Float%20%28single-precision%29)))

(fn ConstructionScript)